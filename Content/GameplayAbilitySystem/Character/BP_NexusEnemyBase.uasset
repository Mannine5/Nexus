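; Base enemy character for the Gameplay Ability System, with a healthbar widget that is removed on death.
; On possession it sends a next-tick gameplay event to equip a ranged staff, then starts a looping attack timer.
; Attack focuses the AI controller on player character 0 and activates a random ability tagged as an AOE attack.
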(event Custom|Attack
  (bind _abilitysystemcomponent (Variables|Default|GetAbilitySystemComponent))
  (bind _attacktarget (CallFunction|GetAttackTarget))
  (AI|SetFocus (AI|GetAIController self) _attacktarget)
  (bind _outabilityhandles (GameplayAbilities|FindAllAbilitieswithTags _abilitysystemcomponent "(GameplayTags=((TagName=\"GameplayAbility.AOEAttack\")))" true))
  (Class|AbilitySystemComponent|TryActivateAbility _abilitysystemcomponent (.OutItem (Utilities|Array|Random _outabilityhandles)) true))

(event EventBeginPlay
  (bind _returnvalue (UserInterface|CreateWidget "/Game/Widgets/Enemy/W_EnemyHealthbar.W_EnemyHealthbar_C" 0 self))
  (UserInterface|SetWidget (Variables|Default|GetHealthbarWidgetComponent) _returnvalue))

(event EventHandleDeath
  (|CallParentFunction)
  (bind _healthbarwidgetcomponent (Variables|Default|GetHealthbarWidgetComponent)
    (:then
      (Components|DestroyComponent _healthbarwidgetcomponent))
    (:else)))

(event EventPossessed
  (params (NewController :type Controller%20Object%20Reference))
  (Utilities|FlowControl|DelayUntilNextTick)
  (Ability|SendGameplayEventtoActor self "(TagName=\"Event.ActivateAbility.EquipWeapon\")" (Utilities|Struct|MakeGameplayEventData "(GameplayTags=((TagName=\"Weapon.Ranged.Staff\")))"))
  (Utilities|Time|SetTimerbyEvent (EventDispatchers|CreateEvent :!event Custom|Attack) 2.0 true))

(fn ConstructionScript)

(fn GetAttackTarget
  (return (Game|GetPlayerCharacter 0)))
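; Base gameplay ability for melee attacks that plays an attack montage using the weapon equipped in the avatar's WeaponsManagerComponent.
; On authority, hit-scan start and end gameplay events open and close the weapon's hit scan, passing it a damage effect spec with a SetByCaller magnitude.
; Montage completion, interruption or cancellation ends the ability, which also closes the hit scan.
; Children can override the empty MontageStarted hook.
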(event Custom|HandleHitScanEnd
  ;[0.15 0.15 0.15 0.5] Hit Scan Events
  (bind _equipped_weapon (Variables|Default|GetEquipped%20Weapon)
    (:then
      (Default|HitScanEnd _equipped_weapon))
    (:else)))

(event Custom|HandleHitScanStart
  (bind _damagemagnitude (Variables|GameplayEffect|GetDamageMagnitude))
  ;[0.15 0.15 0.15 0.5] Hit Scan Events
  (bind _equipped_weapon (Variables|Default|GetEquipped%20Weapon)
    (:then
      (bind _returnvalue (Ability|GameplayEffect|AssignTagSetbyCallerMagnitude (Ability|MakeOutgoingGameplayEffectSpec (Variables|GameplayEffect|GetDamageEffectClass)) "(TagName=\"Data.Damage\")" _damagemagnitude))
      (Default|HitScanStart _equipped_weapon _returnvalue)
      (Development|PrintString (Utilities|String|ToString(Float) _damagemagnitude)))
    (:else)))

(event Custom|MontageStarted
  ;[0.15 0.15 0.15 0.5] Does nothing.
  ; Override in the child.
)

(event Ability|EventActivateAbility
  (bind _returnvalue (Ability|GetAvatarActorfromActorInfo))
  (bind _returnvalue_2 (Actor|GetComponentbyClass _returnvalue "/Game/Assets/Weapons/WeaponsManagerComponent.WeaponsManagerComponent_C"))
  (Utilities|IsValid _returnvalue_2
    (:Is%20Valid
      (bind _equippedweapon (Variables|/Game/Assets/Weapons/WeaponsManagerComponent.WeaponsManagerComponent_C|GetEquippedWeapon _returnvalue_2)
        (:then
          (Variables|Default|SetEquipped%20Weapon _equippedweapon)
          (bind _attackmontage (Variables|Animation|GetAttackMontage)
            (:then
              (|PlayMontageandWaitProxy "None" _attackmontage 1.0 "None" true 1.0 0.0 true
                (:then
                  (CallFunction|MontageStarted)
                  (Ability|HasAuthority
                    (:True
                      (Ability|Tasks|WaitGameplayEvent "(TagName=\"Event.HitScan.Start\")" 0
                        (:then
                          (Ability|Tasks|WaitGameplayEvent "(TagName=\"Event.HitScan.End\")" 0
                            (:EventReceived
                              (CallFunction|HandleHitScanEnd))))
                        (:EventReceived
                          (CallFunction|HandleHitScanStart))))))
                (:OnCompleted
                  (Ability|EndAbility :!label _label))
                (:OnInterrupted
                  (goto _label))
                (:OnCancelled
                  (goto _label))))
            (:else
              (Ability|EndAbility :!label _label_2))))
        (:else
          (goto _label_2))))
    (:Is%20Not%20Valid
      (goto _label_2))))

(event Ability|EventOnEndAbility
  (params (bWasCancelled :type Boolean))
  (CallFunction|HandleHitScanEnd))
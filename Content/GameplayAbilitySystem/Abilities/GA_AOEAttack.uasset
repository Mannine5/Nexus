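; Gameplay ability for an area-of-effect attack on a ground location.
; Uses the ground beneath the avatar's supplied attack target, otherwise lets a player confirm a decal ground-trace target during a looping targeting montage.
; On commit, shows an indicator cue and plays the trigger montage, whose event fires the strike cue.
; After a short delay, the authority sphere-traces pawns, excluding the caster, and applies SetByCaller damage once per actor.
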(event Custom|LoopTargetingAnimation
  ;[0.15 0.15 0.15 0.5] Phase 1
  (|PlayMontageandWaitProxy "None" "/Game/GameplayAbilitySystem/Character/Animations/Staff/Montage_AOE_Targeting.Montage_AOE_Targeting" 1.0 "None" true 1.0 0.0 false
    (:OnBlendOut
      (if (Variables|Default|GetIsWaitingTargetData)
        (CallFunction|LoopTargetingAnimation)))
    (:OnInterrupted
      (if (Variables|Default|GetIsWaitingTargetData)
        (Ability|EndAbility)))))

(event Custom|ConfirmStrike
  ;[0.15 0.15 0.15 0.5] Phase 2
  (bind _returnvalue (Ability|CommitAbility))
  (if _returnvalue
    (Class|GameplayAbility|AddGameplayCuewithParams "(TagName=\"GameplayCue.AOEIndicator\")" (Ability|GameplayCue|MakeGameplayCueParameters :RawMagnitude (Variables|Default|GetAOERadius) :Location (Variables|Default|GetConfirmedAOELocation)) true)
    (|PlayMontageandWaitProxy "None" "/Game/GameplayAbilitySystem/Character/Animations/Staff/Montage_AOE_Trigger.Montage_AOE_Trigger" 1.0 "None" true 1.0 0.0 false
      (:then
        (Ability|Tasks|WaitGameplayEvent "(TagName=\"Event.Montage.Trigger\")" 0
          (:EventReceived
            (Class|GameplayAbility|ExecuteGameplayCuewithParams "(TagName=\"GameplayCue.AOEStrike\")" (Ability|GameplayCue|MakeGameplayCueParameters :Location (Variables|Default|GetConfirmedAOELocation)))
            (Utilities|FlowControl|Delay 0.2)
            (CallFunction|AOEDamage)
            (GameplayCue|RemoveGameplayCue "(TagName=\"GameplayCue.AOEIndicator\")"))))
      (:OnCompleted
        (Ability|EndAbility :!label _label))
      (:OnInterrupted
        (goto _label)))
    (else
      (Ability|EndAbility))))

(event Custom|AOEDamage
  (bind _confirmedaoelocation (Variables|Default|GetConfirmedAOELocation))
  ;[0.15 0.15 0.15 0.5] Phase 2
  (Ability|HasAuthority
    (:True
      (bind _outhits (Collision|MultiSphereTraceForObjects _confirmedaoelocation _confirmedaoelocation (Variables|Default|GetAOERadius) (Utilities|Array|MakeArray "ObjectTypeQuery3") false (Utilities|Array|MakeArray (Ability|GetAvatarActorfromActorInfo)) "ForDuration"))
      (Utilities|Array|Clear (Variables|Default|GetHitActors))
      (for _array_element _outhits
        (if (not (Utilities|Array|ContainsItem (Variables|Default|GetHitActors) (.HitActor (Collision|BreakHitResult _array_element))))
          (Utilities|Array|AddUnique (Variables|Default|GetHitActors) (.HitActor (Collision|BreakHitResult _array_element)))
          (Utilities|IsValid (Ability|GetAbilitySystemComponent (.HitActor (Collision|BreakHitResult _array_element)))
            (:Is%20Valid
              (bind _returnvalue (Ability|GameplayEffect|AssignTagSetbyCallerMagnitude (Ability|MakeOutgoingGameplayEffectSpec "/Game/GameplayAbilitySystem/Effects/GA_AOEDamage_Instant.GA_AOEDamage_Instant_C") "(TagName=\"Data.Damage\")" (Variables|Default|GetDamageMagnitude)))
              (GameplayEffects|ApplyGameplayEffectSpecToSelf (Ability|GetAbilitySystemComponent (.HitActor (Collision|BreakHitResult _array_element))) _returnvalue))))))))

(event Custom|StartTargeting
  ;[0.15 0.15 0.15 0.5] Phase 1
  (if (Class|NexusGameplayAbility|HasPC)
    (CallFunction|LoopTargetingAnimation)
    (Variables|Default|SetIsWaitingTargetData true)
    (bind _data (|WaitTargetData :ConfirmationType "UserConfirmed" :Class "/Game/GameplayAbilitySystem/TargetingActors/GATargetActor_GroundTrace_Decal.GATargetActor_GroundTrace_Decal_C" :DecalSize (Variables|Default|GetAOERadius) :DecalMaterial "/Game/VFX/Decal_AOE.Decal_AOE" :MaxRange 8e+02 :StartLocation (Class|GameplayAbility|MakeTargetLocationInfofromOwnerActor) :ReticleClass 0)
      (:ValidData
        (Variables|Default|SetIsWaitingTargetData false)
        (Variables|Default|SetConfirmedAOELocation (.Location (Collision|BreakHitResult (Ability|TargetData|GetHitResultfromTargetData _data))))
        (CallFunction|ConfirmStrike)))
    (else
      (Ability|EndAbility))))

(event Ability|EventActivateAbility
  ;[0.15 0.15 0.15 0.5] Phase 1
  (bind _attacktarget (Class|BPITargeting|GetAttackTarget(Message) (Ability|GetAvatarActorfromActorInfo)))
  (Utilities|IsValid _attacktarget
    (:Is%20Valid
      (bind _location (CallFunction|GetTargetGroundLocation _attacktarget))
      (Variables|Default|SetConfirmedAOELocation _location)
      (CallFunction|ConfirmStrike))
    (:Is%20Not%20Valid
      (CallFunction|StartTargeting))))

(fn GetTargetGroundLocation
  (params (AttackTarget :type Actor%20Object%20Reference))
  (bind _returnvalue (Transformation|GetActorLocation AttackTarget))
  (bind (_outhit _returnvalue_2) (Collision|LineTraceByChannel _returnvalue (- _returnvalue "0.000000,0.000000,9999.000000") "TraceTypeQuery1" false (Utilities|Array|MakeArray AttackTarget) "None"))
  (return (.Location (Collision|BreakHitResult _outhit)) _returnvalue_2))
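; Gameplay ability that makes a vending machine dispense a soda can, run with BP_VendingMachine as the avatar actor.
; After committing, it waits on a StartVendingAndWait task, firing the Vending.Start gameplay cue when vending starts.
; On completion, a SpawnActor task creates BP_SodaCan at the machine's VendingPoint, then the ability ends.
; A failed commit or cast ends it immediately, while cancellation only prints a message.
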(event Ability|EventActivateAbility
  (bind _returnvalue (Ability|CommitAbility))
  (if _returnvalue
    (bind _asbp_vending_machine (Utilities|Casting|CastToBP_VendingMachine (Ability|GetAvatarActorfromActorInfo))
      (:then
        (|StartVendingandWait _asbp_vending_machine
          (:OnVendingStarted
            (GameplayCue|ExecuteGameplayCue :GameplayCueTag "(TagName=\"GameplayCue.Vending.Start\")"))
          (:OnVendingComplete
            (|SpawnActor 0 (Transformation|GetWorldLocation (Variables|/Game/BluePrints/VendingMachine/BP_VendingMachine.BP_VendingMachine_C|GetVendingPoint _asbp_vending_machine)) "0, 0, 0" "/Game/BluePrints/VendingMachine/BP_SodaCan.BP_SodaCan_C" false 0
              (:then
                (Ability|EndAbility))
              (:Success
                (Development|PrintString "Soda spawn success!"))
              (:DidNotSpawn
                (Development|PrintString "Soda spawn failed!"))))
          (:OnCanceled
            (Development|PrintString "Vending Canceled!"))))
      (:CastFailed
        (Ability|EndAbility :!label _label)))
    (else
      (goto _label))))

(event Ability|EventOnEndAbility
  (params (bWasCancelled :type Boolean)))
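; BP_VendingMachine is a vending machine actor that uses the Gameplay Ability System to trigger its Coke vending ability automatically.
; On the server, Tick passes through a DoOnce that tries to activate GA_CokeVending, then resets after a delay, making a repeating timed attempt.
; Disconnected leftover nodes would grant the ability and print Coke stock from the BeverageSet attributes, but never run.
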(event EventBeginPlay)

(event Collision|EventActorBeginOverlap
  (params (OtherActor :type Actor%20Object%20Reference)))

(event EventTick
  (params (DeltaSeconds :type Float%20%28single-precision%29))
  (Utilities|FlowControl|Sequence
    (:then_0
      (Networking|SwitchHasAuthority
        (:Authority
          (Utilities|FlowControl|DoOnce false :!label _label
            (:Completed
              (Abilities|TryActivateAbilitybyClass (Variables|Default|GetAbilitySystemComponent) "/Game/GameplayAbilitySystem/Abilities/Karelia/GA_CokeVending.GA_CokeVending_C" true)
              (Utilities|FlowControl|Delay 2.0)
              (goto _label Reset))))))))

(fn ConstructionScript)
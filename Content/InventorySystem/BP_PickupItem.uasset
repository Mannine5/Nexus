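; BP_PickupItem is a world pickup actor that grants an inventory item to whatever overlaps it.
; Its construction script reads the WorldRepresentation fragment from the ItemDefinition class to set the static mesh and its scale.
; On overlap, it adds the ItemDefinition to the other actor's InventoryManagerComponent, then destroys itself; actors without that component are ignored.
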(event Collision|EventActorBeginOverlap
  (params (OtherActor :type Actor%20Object%20Reference))
  (bind _returnvalue (Actor|GetComponentbyClass OtherActor "/Game/InventorySystem/InventoryManagerComponent.InventoryManagerComponent_C"))
  (Utilities|IsValid _returnvalue
    (:Is%20Valid
      (Default|AddItem _returnvalue (Variables|Default|GetItemDefinition))
      (Actor|DestroyActor))))

(fn ConstructionScript
  (bind _itemdefinition (Variables|Default|GetItemDefinition))
  (bind _staticmesh (Variables|Default|GetStaticMesh))
  (bind _returnvalue (Class|ItemDefinition|FindFragmentbyClass _itemdefinition "/Script/Nexus.InventoryItemFragment_WorldRepresentation"))
  (Utilities|IsValid _returnvalue
    (:Is%20Valid
      (Components|StaticMesh|SetStaticMesh _staticmesh (Variables|/Script/Nexus.InventoryItemFragment_WorldRepresentation|GetItemMesh _returnvalue))
      (Transformation|SetRelativeScale3D _staticmesh (Variables|/Script/Nexus.InventoryItemFragment_WorldRepresentation|GetMeshScale _returnvalue)))))